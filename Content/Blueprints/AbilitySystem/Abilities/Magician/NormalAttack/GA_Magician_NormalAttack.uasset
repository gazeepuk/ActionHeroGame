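; Gameplay ability for the Magician's normal attack, which fires a projectile from the character toward the camera's aim.
; AbilityAction waits for the Magician normal-attack gameplay event, then traces from the right-hand socket to the camera view, ignoring the caster.
; The hit result yields the transform for spawning the configured projectile class, which carries a gameplay effect spec and spawns only on the server.
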(event Ability|EventActivateAbility
  (|CallParentFunction) ; This node is disabled and will not be called.\nDrag off pins to build functionality.
)

(event Ability|EventOnEndAbility
  (params (bWasCancelled :type Boolean))
  (|CallParentFunction bWasCancelled) ; This node is disabled and will not be called.\nDrag off pins to build functionality.
)

(event EventAbilityAction
  (bind _returnvalue (Class|ActionGameplayAbility|GetActionCharacterfromAvatarActor))
  (Ability|Tasks|WaitGameplayEvent "(TagName=\"Event.Ability.NormalAttack.Magician\")" 0
    (:EventReceived
      (bind _outhitresult (Class|ActionCharacterBase|TraceSingleHitResultfromLocationtoCameraView _returnvalue (Transformation|GetSocketLocation (Variables|/Script/Engine.Character|GetMesh _returnvalue) "RightHandSocket") true (Utilities|Array|MakeArray _returnvalue) 5e+04))
      (bind _returnvalue_2 (Class|ActionFunctionLibrary|GetHitTransformifExist _outhitresult))
      (Class|ActionGameplayAbility|SpawnProjectilebyClass (Variables|Default|GetProjectileClass) _returnvalue_2 3e+03 0.0 (Utilities|Struct|MakeGameplayEffectSpec) true))))